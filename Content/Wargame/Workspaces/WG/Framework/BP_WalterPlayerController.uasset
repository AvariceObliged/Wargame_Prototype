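; Player controller for a wargame that selects a model pawn and orders range-limited moves with the mouse.
; Right-click stores the BP_WalterModelPawn under the cursor as TargetModel.
; Tick finds a navmesh path to the cursor, debug-drawing it green within MaxLength and red beyond, interpolating the cutoff point as Destination.
; Left-click sends the model there via AIMoveTo, with CanMove blocking preview and new orders until the move succeeds or fails.
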(event `Key|RightMouseButton`
  (params (Key :type "Key Structure"))
  (:`Pressed`
    (bind (_hit _model) (`self.GetModelUnderCursor`))
    (bind _output_get (set `self.TargetModel` _model))
    (`KismetSystemLibrary.PrintString` (`KismetSystemLibrary.GetDisplayName` _output_get))))

(event `self.ReceiveTick`
  (params (DeltaSeconds :type "Float (single-precision)"))
  (if (and (`self.IsTargetModelValid`) (`self.CanMove`))
    (bind (_hit _location) (`self.GetLocationUnderCursor`))
    (if _hit
      (bind _returnvalue (`NavigationSystemV1.FindPathToLocationSynchronously` (`self.TargetModelLocation`) _location (`self.TargetModel`) null))
      (set `self.CurrentLength` 0.0)
      (bind _output_get (set `self.HasDestination` (> (`NavigationPath.GetPathLength` _returnvalue) 0.0)))
      (if _output_get
        (bind _pathpoints (`NavigationPath.PathPoints` _returnvalue))
        (for (_array_element _array_index) _pathpoints
          (switch `int` _array_index
            (:`Default`
              (if (> (`self.CurrentLength`) (`self.MaxLength`))
                (bind _output (`|GetArrayItem` _pathpoints (- _array_index 1)))
                (`KismetSystemLibrary.DrawDebugLine` _output _array_element (struct :`R` 0.75 :`A` 1.0) 0.0 20.0)
                (else
                  (bind _returnvalue_2 (`KismetMathLibrary.VSize` (- _output _array_element)))
                  (bind _returnvalue_3 (+ (`self.CurrentLength`) _returnvalue_2))
                  (if (<= _returnvalue_3 (`self.MaxLength`))
                    (`KismetSystemLibrary.DrawDebugLine` _output _array_element (struct :`G` 0.75 :`B` 0.054644 :`A` 1.0) 0.0 20.0)
                    (set `self.Destination` _array_element)
                    (else
                      (bind _returnvalue_4 (`KismetMathLibrary.VLerp` _output _array_element (/ (- (`self.MaxLength`) (`self.CurrentLength`)) _returnvalue_2)))
                      (`KismetSystemLibrary.DrawDebugLine` _output _returnvalue_4 (struct :`G` 0.75 :`B` 0.054644 :`A` 1.0) 0.0 20.0)
                      (`KismetSystemLibrary.DrawDebugLine` _array_element _returnvalue_4 (struct :`R` 0.75 :`A` 1.0) 0.0 20.0)
                      (set `self.Destination` _returnvalue_4)))))
              (set `self.CurrentLength` _returnvalue_3)))))
      (else
        (set `self.HasDestination` false)))
    (else
      (set `self.HasDestination` false))))

(event `Key|LeftMouseButton`
  (params (Key :type "Key Structure"))
  (:`Pressed`
    (if (and (`self.IsTargetModelValid`) (`self.HasDestination`) (`self.CanMove`))
      (set `self.CanMove` false)
      (`|AIMoveTo` (`self.TargetModel`) (`self.Destination`) null
        (:`OnSuccess`
          _)
        (:`OnFail`
          _))
      (set `self.CanMove` true))))

(fn `GetLocationUnderCursor`
  (returns (Hit :type Boolean) (Location :type "Vector Structure"))
  (bind (_bblockinghit _binitialoverlap _time _distance _location) (`GameplayStatics.BreakHitResult` (`self.GetHitResultUnderCursorByChannel` "TraceTypeQuery1")))
  (return _bblockinghit _location))

(fn `GetModelUnderCursor`
  (returns (Hit :type Boolean) (Model :type "/Game/Wargame/Workspaces/WG/Blueprints/BP_WalterModelPawn Object Reference"))
  (bind _asbp_walter_model_pawn (cast `/Game/Wargame/Workspaces/WG/Blueprints/BP_WalterModelPawn` (`.HitActor` (`GameplayStatics.BreakHitResult` (`self.GetHitResultUnderCursorByChannel` "TraceTypeQuery1"))))
    (:`then`
      _)
    (:`CastFailed`
      _))
  (return (`KismetSystemLibrary.IsValid` _asbp_walter_model_pawn) _asbp_walter_model_pawn))

(fn `UserConstructionScript`)