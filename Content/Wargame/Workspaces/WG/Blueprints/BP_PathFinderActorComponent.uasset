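; BP_PathFinderActorComponent is an actor component that computes and stores a navigation path for its owning actor.
; Find Path runs a synchronous navmesh query from the owner's location to a target, stores the resulting points in PathPoints, and fires a path-found notification.
; Clear Path empties the stored points and fires a path-cleared notification.
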(fn `Clear Path`
  (`KismetArrayLibrary.Array_Clear` (`self.Path Points`))
  (`self.Path Cleared`))

(fn `Find Path`
  (params (Target :type "Vector Structure"))
  (bind _returnvalue (`NavigationSystemV1.FindPathToLocationSynchronously` (`self.Actor Location`) Target null null))
  (set `self.Path Points` (`NavigationPath.PathPoints` _returnvalue))
  (`self.Path Found`))