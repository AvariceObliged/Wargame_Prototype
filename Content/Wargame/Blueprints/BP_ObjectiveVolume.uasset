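; Objective volume for a wargame that totals victory points per player from the models standing inside it.
; Begin and end overlaps with a BP_ModelActor rebuild the set of scoring models from the collision component's overlapping actors.
; Each model's ModelBP supplies its owning player ID and victory points, which are summed into a PointsPerPlayer map.
; GetScoresByPlayerID runs the same refresh before returning that map.
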(event `self.ReceiveActorBeginOverlap`
  (params (OtherActor :type "Actor Object Reference"))
  ;[1 1 1] Update values only if overlapping actor is A Model_Actor
  (if (`GameplayStatics.ObjectIsA` OtherActor "/Game/Wargame/Blueprints/BP_ModelActor.BP_ModelActor_C")
    (`self.UpdateValues`)))

(event `self.ReceiveActorEndOverlap`
  (params (OtherActor :type "Actor Object Reference"))
  ;[1 1 1] Update values only if overlapping actor is A Model_Actor
  (if (`GameplayStatics.ObjectIsA` OtherActor "/Game/Wargame/Blueprints/BP_ModelActor.BP_ModelActor_C")
    (`self.UpdateValues`)))

(fn `GetScoresByPlayerID`
  (returns (`Points By Player ID` :type "Map of Integer to Integer"))
  (`self.Update All Scoring Models`)
  (`self.Update Points Per Player`)
  (return (`self.PointsPerPlayer`)))

(fn `Update All Scoring Models`
  (locals (TempScoringModels :type "Array of /Game/Wargame/Blueprints/BP_ModelActor Object Reference"))
  (`BlueprintSetLibrary.Set_Clear` (`self.AllScoringModels`))
  (for _array_element (`PrimitiveComponent.GetOverlappingActors` (`self.CollisionComponent`) "/Game/Wargame/Blueprints/BP_ModelActor.BP_ModelActor_C")
    (bind _asbp_model_actor (cast `/Game/Wargame/Blueprints/BP_ModelActor` _array_element))
    (`KismetArrayLibrary.Array_Add` (`local.TempScoringModels`) _asbp_model_actor))
  (`BlueprintSetLibrary.Set_AddItems` (`self.AllScoringModels`) (`local.TempScoringModels`)))

(fn `Update Points Per Player`
  (locals (`Local Owning Player ID` :type Integer) (`Local Victory Points` :type Integer))
  (`BlueprintMapLibrary.Map_Clear` (`self.PointsPerPlayer`))
  (bind _result (`BlueprintSetLibrary.Set_ToArray` (`self.AllScoringModels`)))
  (for _array_element _result
    (bind _modelbp (`/Game/Wargame/Blueprints/BP_ModelActor.ModelBP` _array_element))
    (set `local.Local Owning Player ID` (`/Game/Wargame/Blueprints/BP_Model.OwningPlayerID` _modelbp))
    (set `local.Local Victory Points` (`/Game/Wargame/Blueprints/BP_Model.VictoryPoints` _modelbp))
    (bind _keys (`BlueprintMapLibrary.Map_Keys` (`self.PointsPerPlayer`)))
    (if (`KismetArrayLibrary.Array_Contains` _keys (`local.Local Owning Player ID`))
      (`BlueprintMapLibrary.Map_Add` (`self.PointsPerPlayer`) (`local.Local Owning Player ID`) (+ (`BlueprintMapLibrary.Map_Find` (`self.PointsPerPlayer`) (`local.Local Owning Player ID`)) (`local.Local Victory Points`)))
      (else
        (`BlueprintMapLibrary.Map_Add` (`self.PointsPerPlayer`) (`local.Local Owning Player ID`) (`local.Local Victory Points`))))))

(fn `UpdateValues`
  (`self.Update All Scoring Models`)
  (`self.Update Points Per Player`))

(fn `UserConstructionScript`)