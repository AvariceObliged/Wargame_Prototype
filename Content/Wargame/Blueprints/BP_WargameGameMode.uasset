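; Game mode for a turn-based multiplayer wargame, managing turn order and each player's order points.
; PostLogin seeds controllers with starting points and starts the game once two or more players are present.
; Each turn cycle advances the wrapping active-player index, grants per-turn points and notifies controllers through CLIENT-suffixed events.
; Spawns come from a lazily built map of BP_WargamePlayerStart actors by player index, looked up by current player count.
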(event `self.K2_PostLogin`
  (params (NewPlayer :type "PlayerController Object Reference"))
  (bind _returnvalue (`self.GetNumPlayers`))
  (for _index (range (+ _returnvalue 1))
    (bind _asbp_wargame_controller (cast `/Game/Wargame/Blueprints/BP_WargameController` (`GameplayStatics.GetPlayerController` _index)))
    (`BlueprintMapLibrary.Map_Add` (`self.PlayerOrderPoints`) _asbp_wargame_controller (`self.StartingOrderPoints`)))
  (if (>= _returnvalue 2)
    (`self.StartGame`)))

(event `StartGame`
  (bind _activeplayercontroller (`self.GetActivePlayer`))
  (`self.IncrementActivePlayersOrderPoints`)
  (bind _order_points (`self.Get Order Points by Player Controller` _activeplayercontroller))
  (`/Game/Wargame/Blueprints/BP_WargameController.UpdateOrderPoints_CLIENT` _activeplayercontroller _order_points)
  (`/Game/Wargame/Blueprints/BP_WargameController.StartTurn_CLIENT` _activeplayercontroller))

(event `CycleTurns`
  (bind _activeplayercontroller (`self.GetActivePlayer`))
  (`/Game/Wargame/Blueprints/BP_WargameController.EndTurn_CLIENT` (`self.GetActivePlayer`))
  (`self.IncrementActivePlayerIndex`)
  (`self.IncrementActivePlayersOrderPoints`)
  (bind _order_points (`self.Get Order Points by Player Controller` _activeplayercontroller))
  (`/Game/Wargame/Blueprints/BP_WargameController.UpdateOrderPoints_CLIENT` _activeplayercontroller _order_points)
  (`/Game/Wargame/Blueprints/BP_WargameController.StartTurn_CLIENT` (`self.GetActivePlayer`)))

(fn `ChoosePlayerStart`
  (params (Player :type "Controller Object Reference"))
  (returns (ReturnValue :type "Actor Object Reference"))
  (`self.InitializeSpawnPoints`)
  (bind _returnvalue (`self.GetNumPlayers`))
  (return (`BlueprintMapLibrary.Map_Find` (`self.SpawnPoints`) _returnvalue)))

(fn `Get Order Points by Player Controller`
  (params (`Player Controller` :type "/Game/Wargame/Blueprints/BP_WargameController Object Reference"))
  (returns (`Order Points` :type Integer))
  (bind (_value _returnvalue) (`BlueprintMapLibrary.Map_Find` (`self.PlayerOrderPoints`) `Player Controller`))
  (if _returnvalue
    (return _value)
    (else
      (`KismetSystemLibrary.PrintString` "ERR: index missing")
      (return -1))))

(fn `IncrementActivePlayerIndex`
  (if (>= (`self.ActivePlayerIndex`) (- (`self.NumPlayers`) 1))
    (set `self.ActivePlayerIndex` 0)
    (else
      (set `self.ActivePlayerIndex` (+ 1 (`self.ActivePlayerIndex`))))))

(fn `IncrementActivePlayersOrderPoints`
  (`BlueprintMapLibrary.Map_Add` (`self.PlayerOrderPoints`) (`self.GetActivePlayer`) (+ (`BlueprintMapLibrary.Map_Find` (`self.PlayerOrderPoints`) (`self.GetActivePlayer`)) (`self.OrderPointsPerTurn`))))

(fn `InitializeSpawnPoints`
  (if (== 0 (`BlueprintMapLibrary.Map_Length` (`self.SpawnPoints`)))
    (bind _outactors (`GameplayStatics.GetAllActorsOfClass` "/Game/Wargame/Blueprints/BP_WargamePlayerStart.BP_WargamePlayerStart_C"))
    (for _array_element _outactors
      (`BlueprintMapLibrary.Map_Add` (`self.SpawnPoints`) (`/Game/Wargame/Blueprints/BP_WargamePlayerStart.GetPlayerIndex` _array_element) _array_element))))

(fn `UserConstructionScript`)