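; Objective component for a wargame that tallies victory points per player from the models standing on its owner.
; It gathers BP_ModelActors overlapping the owner's shape component into a scoring set, then sums their victory points into a map keyed by owning player ID.
; GetScoresByPlayerID and UpdateValues both run this update, the former returning the map.
; The owner's W_ObjectiveDisplay widget receives the map during gathering, before the totals are recalculated.
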(fn `GetScoresByPlayerID`
  (returns (PointsByPlayerID :type "Map of Integer to Integer"))
  (`self.UpdateAllScoringModels`)
  (`self.UpdatePointsPerPlayer`)
  (return (`self.PointsPerPlayer`)))

(fn `UpdateAllScoringModels`
  (locals (TempScoringModels :type "Array of /Game/Wargame/Blueprints/Actors/BP_ModelActor Object Reference"))
  (`BlueprintSetLibrary.Set_Clear` (`self.AllScoringModels`))
  (for _array_element (`PrimitiveComponent.GetOverlappingActors` (`Actor.GetComponentByClass` (`self.GetOwner`) "/Script/Engine.ShapeComponent") "/Game/Wargame/Blueprints/Actors/BP_ModelActor.BP_ModelActor_C")
    (bind _asbp_model_actor (cast `/Game/Wargame/Blueprints/Actors/BP_ModelActor` _array_element))
    (`KismetArrayLibrary.Array_Add` (`local.TempScoringModels`) _asbp_model_actor))
  (`BlueprintSetLibrary.Set_AddItems` (`self.AllScoringModels`) (`local.TempScoringModels`))
  (bind _asw_objective_display (cast `/Game/Wargame/UI/Objective/W_ObjectiveDisplay` (`WidgetComponent.GetWidget` (`Actor.GetComponentByClass` (`self.GetOwner`) "/Script/UMG.WidgetComponent"))))
  (`/Game/Wargame/UI/Objective/W_ObjectiveDisplay.PopulateScoreListView` _asw_objective_display (`self.PointsPerPlayer`)))

(fn `UpdatePointsPerPlayer`
  (locals (LocalOwningPlayerID :type Integer) (LocalVictoryPoints :type Integer))
  (`BlueprintMapLibrary.Map_Clear` (`self.PointsPerPlayer`))
  (bind _result (`BlueprintSetLibrary.Set_ToArray` (`self.AllScoringModels`)))
  (for _array_element _result
    (bind _modelbp (`/Game/Wargame/Blueprints/Actors/BP_ModelActor.ModelBP` _array_element))
    (set `local.LocalOwningPlayerID` (`/Game/Wargame/Blueprints/Components/BP_Model.OwningPlayerID` _modelbp))
    (set `local.LocalVictoryPoints` (`/Game/Wargame/Blueprints/Components/BP_Model.VictoryPoints` _modelbp))
    (bind _keys (`BlueprintMapLibrary.Map_Keys` (`self.PointsPerPlayer`)))
    (if (`KismetArrayLibrary.Array_Contains` _keys (`local.LocalOwningPlayerID`))
      (`BlueprintMapLibrary.Map_Add` (`self.PointsPerPlayer`) (`local.LocalOwningPlayerID`) (+ (`BlueprintMapLibrary.Map_Find` (`self.PointsPerPlayer`) (`local.LocalOwningPlayerID`)) (`local.LocalVictoryPoints`)))
      (else
        (`BlueprintMapLibrary.Map_Add` (`self.PointsPerPlayer`) (`local.LocalOwningPlayerID`) (`local.LocalVictoryPoints`))))))

(fn `UpdateValues`
  (`self.UpdateAllScoringModels`)
  (`self.UpdatePointsPerPlayer`))