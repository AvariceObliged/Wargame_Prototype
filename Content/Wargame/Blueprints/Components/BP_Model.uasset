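; BP_Model is a wargame Blueprint that holds a model's name and its collection of weapon profiles.
; GetWeaponProfile converts the collection to an array, then prints the name of the first entry and returns it if one exists.
; GetModelName only prints the stored name, while both setters and the BeginPlay and Tick events are empty stubs.
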(event `self.ReceiveBeginPlay`)

(event `self.ReceiveTick`
  (params (DeltaSeconds :type "Float (single-precision)")))

(fn `GetModelName`
  (`KismetSystemLibrary.PrintString` (`self.ModelName`)))

(fn `GetWeaponProfile`
  (returns (`Current WP` :type "/Game/Wargame/Blueprints/Components/BP_WeaponProfile Object Reference"))
  (bind _result (`BlueprintSetLibrary.Set_ToArray` (`self.WeaponProfiles`)))
  (if (`KismetArrayLibrary.Array_IsValidIndex` _result)
    (bind _output (`|GetArrayItem` _result))
    (`KismetSystemLibrary.PrintString` (`/Game/Wargame/Blueprints/Components/BP_WeaponProfile.WeaponProfileName` _output))
    (return _output)
    (else
      (return null))))

(fn `SetModelName`)

(fn `SetWeaponProfile`)