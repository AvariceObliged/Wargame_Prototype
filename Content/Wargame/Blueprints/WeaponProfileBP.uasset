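; WeaponProfileBP is a wargame weapon profile that holds a name, accuracy, strength, save penetration, damage and range limits.
; Two debug functions print this data to screen, one for the name alone and one for each labelled stat.
; BeginPlay only reassigns the profile name to itself, and no combat logic is present.
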(event `self.ReceiveBeginPlay`
  (set `self.WeaponProfileName` (`self.WeaponProfileName`)))

(fn `PrintWPName`
  (`KismetSystemLibrary.PrintString` (`self.WeaponProfileName`)))

(fn `PrintWPNStats`
  (`KismetSystemLibrary.PrintString` (`KismetStringLibrary.Concat_StrStr` "Name " (`KismetSystemLibrary.MakeLiteralString` (`self.WeaponProfileName`))))
  (`KismetSystemLibrary.PrintString` (`KismetStringLibrary.Concat_StrStr` "Accuracy " (`KismetSystemLibrary.MakeLiteralString` (`KismetStringLibrary.Conv_IntToString` (`self.accuracy`)))))
  (`KismetSystemLibrary.PrintString` (`KismetStringLibrary.Concat_StrStr` "Strength " (`KismetSystemLibrary.MakeLiteralString` (`KismetStringLibrary.Conv_IntToString` (`self.strength`)))))
  (`KismetSystemLibrary.PrintString` (`KismetStringLibrary.Concat_StrStr` "Save Pen " (`KismetSystemLibrary.MakeLiteralString` (`KismetStringLibrary.Conv_IntToString` (`self.savePenetration`)))))
  (`KismetSystemLibrary.PrintString` (`KismetStringLibrary.Concat_StrStr` "Damage " (`KismetSystemLibrary.MakeLiteralString` (`KismetStringLibrary.Conv_IntToString` (`self.damage`)))))
  (`KismetSystemLibrary.PrintString` (`KismetStringLibrary.Concat_StrStr` "Min Range " (`KismetSystemLibrary.MakeLiteralString` (`KismetStringLibrary.Conv_IntToString` (`self.minRange`)))))
  (`KismetSystemLibrary.PrintString` (`KismetStringLibrary.Concat_StrStr` "Max Range " (`KismetSystemLibrary.MakeLiteralString` (`KismetStringLibrary.Conv_IntToString` (`self.maxRange`))))))