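; Player controller for a turn-based multiplayer wargame, tracking whether this player is active and adding the turn status widget and input mapping context.
; Client events set turn state and broadcast active-player and order-point changes through dispatchers.
; Server events route move, attack and ability costs and turn cycling to BP_WargameGameMode.
; Left-click release is gated on the active turn, but its handler is still empty.
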(event `self.ReceiveBeginPlay`
  (bind _returnvalue (subsystem `EnhancedInputLocalPlayerSubsystem`))
  (if (`self.IsLocalController` self)
    (bind _returnvalue_2 (`|CreateWidget` "/Game/Wargame/UI/BP_TurnStatusWidget.BP_TurnStatusWidget_C" self))
    (`UserWidget.AddToViewport` _returnvalue_2 0))
  (`/Engine/EditorBlueprintResources/StandardMacros.IsValid` _returnvalue
    (:`Is Valid`
      (`EnhancedInputSubsystemInterface.AddMappingContext` _returnvalue "/Game/Wargame/Input/IMC_Default.IMC_Default" 0 (struct)))))

(event `SetMyTurn_CLIENT`
  (`self.SetActivePlayer` true))

(event `UpdateOrderPoints_CLIENT`
  (params (OrderPoints :type Integer))
  (`self.OnOrderPointsChanged` OrderPoints))

(event `SetTurnOver_CLIENT`
  (`KismetSystemLibrary.PrintString` "Ending Turn")
  (`self.SetActivePlayer` false))

(event `Key|LeftMouseButton`
  (params (Key :type "Key Structure"))
  (:`Released`
    (if (`self.ActivePlayer`)
      (`self.HandleLeftMouseButton`))))

(event `UnitMove_SERVER`
  (bind _asbp_wargame_game_mode (cast `/Game/Wargame/Blueprints/BP_WargameGameMode` (`GameplayStatics.GetGameMode`)))
  (`/Game/Wargame/Blueprints/BP_WargameGameMode.SpendOrderPoints` _asbp_wargame_game_mode (`self.MovementCost`) self))

(event `UnitAttack_SERVER`
  (bind _asbp_wargame_game_mode (cast `/Game/Wargame/Blueprints/BP_WargameGameMode` (`GameplayStatics.GetGameMode`)))
  (`/Game/Wargame/Blueprints/BP_WargameGameMode.SpendOrderPoints` _asbp_wargame_game_mode (`self.AttackCost`) self))

(event `UnitAbility_SERVER`
  (bind _asbp_wargame_game_mode (cast `/Game/Wargame/Blueprints/BP_WargameGameMode` (`GameplayStatics.GetGameMode`)))
  (`/Game/Wargame/Blueprints/BP_WargameGameMode.SpendOrderPoints` _asbp_wargame_game_mode (`self.AbilityCost`) self))

(event `CycleTurn_SERVER`
  (bind _asbp_wargame_game_mode (cast `/Game/Wargame/Blueprints/BP_WargameGameMode` (`GameplayStatics.GetGameMode`)))
  (`/Game/Wargame/Blueprints/BP_WargameGameMode.CycleTurns` _asbp_wargame_game_mode))

(fn `HandleLeftMouseButton`)

(fn `SetActivePlayer`
  (params (Active :type Boolean))
  (bind _output_get (set `self.ActivePlayer` Active))
  (`self.OnActivePlayerChanged` _output_get))

(fn `UserConstructionScript`)