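; Player camera pawn for a wargame, cycling through three numbered camera modes driven by Enhanced Input.
; Crane mode pins movement to a plane through FloatingPawnMovement, with zoom raising or lowering that plane within clamped limits.
; Mode 1 moves freely along local axes, while mode 2 releases the plane but has no movement handler.
; Look input rotates with clamped pitch and recenters the mouse; the look-enable action toggles cursor visibility.
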(event `self.ReceiveBeginPlay`
  (`self.Set Show Mouse Cursor` true)
  (`self.SetCameraModeValue` 0))

(event `EnhancedInput|/Game/Wargame/Input/Actions/IA_CycleCamType`
  (params (ActionValue :type Boolean) (ElapsedSeconds :type "Float (double-precision)") (TriggeredSeconds :type "Float (double-precision)") (InputAction :type "InputAction Object Reference" :default "/Game/Wargame/Input/Actions/IA_CycleCamType.IA_CycleCamType"))
  (:`Triggered`
    (`self.CycleCameraMode`)))

(event `EnhancedInput|/Game/Wargame/Input/Actions/IA_Zoom`
  (params (ActionValue :type "Float (double-precision)") (ElapsedSeconds :type "Float (double-precision)") (TriggeredSeconds :type "Float (double-precision)") (InputAction :type "InputAction Object Reference" :default "/Game/Wargame/Input/Actions/IA_Zoom.IA_Zoom"))
  (:`Triggered`
    (`self.AlterCameraZoom` ActionValue)))

(event `EnhancedInput|/Game/Wargame/Input/Actions/IA_CamLook`
  (params (ActionValue :type "Vector2D Structure") (ElapsedSeconds :type "Float (double-precision)") (TriggeredSeconds :type "Float (double-precision)") (InputAction :type "InputAction Object Reference" :default "/Game/Wargame/Input/Actions/IA_CamLook.IA_CamLook"))
  (:`Triggered`
    (`self.RotateCamera` ActionValue)))

(event `EnhancedInput|/Game/Wargame/Input/Actions/IA_MoveCamera`
  (params (ActionValue :type "Vector2D Structure") (ElapsedSeconds :type "Float (double-precision)") (TriggeredSeconds :type "Float (double-precision)") (InputAction :type "InputAction Object Reference" :default "/Game/Wargame/Input/Actions/IA_MoveCamera.IA_MoveCamera"))
  (:`Triggered`
    (switch `int` (`self.CameraMode`)
      (:`0`
        (`self.CraneCameraMove` ActionValue))
      (:`1`
        (`self.FreeCameraMove` ActionValue)))))

(event `EnhancedInput|/Game/Wargame/Input/Actions/IA_EnableCamLook`
  (params (ActionValue :type Boolean) (ElapsedSeconds :type "Float (double-precision)") (TriggeredSeconds :type "Float (double-precision)") (InputAction :type "InputAction Object Reference" :default "/Game/Wargame/Input/Actions/IA_EnableCamLook.IA_EnableCamLook"))
  (:`Triggered`
    (`self.Set Show Mouse Cursor` (not ActionValue) :!label _label))
  (:`Completed`
    (goto _label)))

(fn `AlterCameraZoom`
  (params (Input :type "Float (double-precision)"))
  (if (== (`self.CameraMode`) 0)
    (`self.Set Plane Constrained True`)
    (`MovementComponent.SetPlaneConstraintOrigin` (`self.FloatingPawnMovement`) (`KismetMathLibrary.MakeVector` 0.0 0.0 (`KismetMathLibrary.FClamp` (+ (* Input 20.0) (`.Z` (`KismetMathLibrary.BreakVector3f` (`MovementComponent.GetPlaneConstraintOrigin` (`self.FloatingPawnMovement`))))) 20.0 10000.0)))
    (`MovementComponent.SnapUpdatedComponentToPlane` (`self.FloatingPawnMovement`))))

(fn `CraneCameraMove`
  (params (A :type "Vector2D Structure"))
  (bind (_x _y) (`KismetMathLibrary.BreakVector2D` (* A (`self.CameraMoveSpeed`))))
  (`self.K2_AddActorLocalOffset` (`KismetMathLibrary.MakeVector` _x _y) true)
  (`MovementComponent.SnapUpdatedComponentToPlane` (`self.FloatingPawnMovement`)))

(fn `CycleCameraMode`
  (bind _camera_mode (`self.IncrementCameraModeValue`))
  (`self.SetCameraModeValue` _camera_mode))

(fn `FreeCameraMove`
  (params (A :type "Vector2D Structure"))
  (bind (_x _y) (`KismetMathLibrary.BreakVector2D` (* A (`self.CameraMoveSpeed`))))
  (`self.K2_AddActorLocalOffset` (`KismetMathLibrary.MakeVector` _x _y) true))

(fn `IncrementCameraModeValue`
  (returns (`Camera Mode` :type Integer))
  (if (>= (`self.CameraMode`) 2)
    (bind _output_get (set `self.CameraMode` 0))
    (else
      (set `self.CameraMode` (+ (`self.CameraMode`) 1))))
  (return _output_get))

(fn `RotateCamera`
  (params (InVector2d :type "Vector2D Structure"))
  (locals (TargetRotation :type "Rotator Structure"))
  (bind (_returnvalue_roll _returnvalue_pitch _returnvalue_yaw) (`KismetMathLibrary.BreakRotator` (`self.K2_GetActorRotation`)))
  (bind (_x _y) (`KismetMathLibrary.BreakVector2D` (* InVector2d (`self.CameraRotationSpeed`))))
  (`self.Set Mouse to Center Screen`
    (:`Out`
      (set `local.TargetRotation` (struct))
      (bind _output_get (set `local.TargetRotation` (`KismetMathLibrary.MakeRotator` 0.0 (`KismetMathLibrary.ClampAngle` (+ _y _returnvalue_pitch) -89.5 89.5) (+ _x _returnvalue_yaw))))
      (`self.K2_SetActorRotation` _output_get)
      (`self.Set Mouse to Center Screen`))))

(fn `SetCameraModeValue`
  (params (`Camera Mode` :type Integer))
  (switch `int` `Camera Mode`
    (:`Default`
      (`self.Set Plane Constrained True` :!label _label)
      (`MovementComponent.SetPlaneConstraintOrigin` (`self.FloatingPawnMovement`) (`self.K2_GetActorLocation`)))
    (:`0`
      (goto _label))
    (:`1`
      (`self.Set Plane Constrained False`)
      (`KismetSystemLibrary.PrintString` (`KismetStringLibrary.BuildString_Int` "Camera Mode: " "" (`self.CameraMode`)) :!label _label_2))
    (:`2`
      (`self.Set Plane Constrained False`)
      (goto _label_2))))

(fn `UserConstructionScript`)