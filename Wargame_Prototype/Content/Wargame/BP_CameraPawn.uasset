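; BP_CameraPawn is a camera pawn for the Wargame that provides smoothed zoom and rotation around a spring arm.
; Each Tick, ZoomCamera and RotateCamera read Enhanced Input action values and lerp persistent rates toward them using delta time, so motion eases in and out.
; The inverted, magnified zoom rate changes the arm length within fixed limits, while the rotation rate adds relative yaw to the arm.
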(event `self.ReceiveTick`
  (params (DeltaSeconds :type "Float (single-precision)"))
  (`self.ZoomCamera`)
  (`self.RotateCamera`))

(fn `RotateCamera`
  (bind _output_get (set `self.RotationRate` (`KismetMathLibrary.Lerp` (`self.RotationRate`) (* (`|GetInputActionValue`) 1.2) (* 5.0 (`GameplayStatics.GetWorldDeltaSeconds`)))))
  (`SceneComponent.K2_AddRelativeRotation` (`self.SpringArm`) (`KismetMathLibrary.MakeRotator` 0.0 0.0 _output_get) false false))

(fn `UserConstructionScript`)

(fn `ZoomCamera`
  (bind _output_get (set `self.ZoomRate` (`KismetMathLibrary.Lerp` (`self.ZoomRate`) (* (`|GetInputActionValue`) -100.0) (* (`GameplayStatics.GetWorldDeltaSeconds`) 5.0))))
  (set `SpringArmComponent.TargetArmLength` (`KismetMathLibrary.FClamp` (+ _output_get (`SpringArmComponent.TargetArmLength` (`self.SpringArm`))) 200.0 10000.0) (`self.SpringArm`)))